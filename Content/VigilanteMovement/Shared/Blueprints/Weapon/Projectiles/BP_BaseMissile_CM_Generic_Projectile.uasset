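; Generic cruise missile projectile Blueprint that animates the deployment of its fins and wing shortly after spawning.
; On BeginPlay it casts the skeletal mesh's anim instance to the BGM109 missile AnimBP, initializes the fin and wing angles, then waits briefly.
; DeployWings plays the SetWings timeline in reverse from its end, feeding the curve into RearFinsAngle and RightWingAngle.
; Both routines set RightWingAngle twice and never set a left wing angle.
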(event `self.ReceiveBeginPlay`
  (`parent.ReceiveBeginPlay`)
  (bind _asabp_west_missile_bgm109 (cast `/Game/VigilanteMovement/Shared/Blueprints/Weapon/Projectiles/Meshes/West_Missile_BGM109/ABP_West_Missile_BGM109` (`SkeletalMeshComponent.GetAnimInstance` (`self.SkeletalMesh`))))
  (set `self.AnimInstance` _asabp_west_missile_bgm109)
  (set `/Game/VigilanteMovement/Shared/Blueprints/Weapon/Projectiles/Meshes/West_Missile_BGM109/ABP_West_Missile_BGM109.RearFinsAngle` 1.0 (`self.AnimInstance`))
  (set `/Game/VigilanteMovement/Shared/Blueprints/Weapon/Projectiles/Meshes/West_Missile_BGM109/ABP_West_Missile_BGM109.RightWingAngle` 1.0 (`self.AnimInstance`))
  (set `/Game/VigilanteMovement/Shared/Blueprints/Weapon/Projectiles/Meshes/West_Missile_BGM109/ABP_West_Missile_BGM109.RightWingAngle` 1.0 (`self.AnimInstance`))
  (`KismetSystemLibrary.Delay` 1.0)
  (`self.DeployWings`))

(event `DeployWings`
  (bind (_direction _cu_smooth_simplecurve) (`Timeline|SetWings` :!via `ReverseFromEnd`)
    (:`Update`
      (bind _output_get (set `/Game/VigilanteMovement/Shared/Blueprints/Weapon/Projectiles/Meshes/West_Missile_BGM109/ABP_West_Missile_BGM109.RearFinsAngle` _cu_smooth_simplecurve (`self.AnimInstance`)))
      (bind _output_get_2 (set `/Game/VigilanteMovement/Shared/Blueprints/Weapon/Projectiles/Meshes/West_Missile_BGM109/ABP_West_Missile_BGM109.RightWingAngle` _output_get (`self.AnimInstance`)))
      (set `/Game/VigilanteMovement/Shared/Blueprints/Weapon/Projectiles/Meshes/West_Missile_BGM109/ABP_West_Missile_BGM109.RightWingAngle` _output_get_2 (`self.AnimInstance`)))))

(fn `UserConstructionScript`
  (`parent.UserConstructionScript`))