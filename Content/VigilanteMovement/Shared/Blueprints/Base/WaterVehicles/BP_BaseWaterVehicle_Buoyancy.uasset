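; Base physics-driven water vehicle with a Buoyancy component, supporting boats and submarines.
; Thrust input accumulates throttle into a speed-limited force on the skeletal mesh, while steering applies yaw impulses scaled by speed.
; Submarines also pitch by impulse and dive by overriding mesh mass as simulated ballast tanks.
; Empty SetThrottle and SetTurn events serve as hooks, and entering water records the surface height.
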(event `self.ReceiveBeginPlay`
  (`parent.ReceiveBeginPlay`)
  ;[1 1 1] Sets Physics Maximal Rotation Velocity
  (`PrimitiveComponent.SetPhysicsMaxAngularVelocityInDegrees` (`self.SkeletalMesh`) (`self.TurnMaxAngVel`) false "None"))

(event `self.ReceiveTick`
  (params (DeltaSeconds :type "Float (single-precision)"))
  (`parent.ReceiveTick` DeltaSeconds))

(event `UpdateThrottle`
  (params (Value :type "Float (double-precision)"))
  ;[1 1 1] Updates Throttle
  (set `self.Throttle` (`KismetMathLibrary.FClamp` (+ (* Value (`self.ThrottleRate`)) (`self.Throttle`)) -1.0))
  (`self.UpdateSpeed`)
  (`self.SetThrottle`))

(event `SetThrottle`
  ;[1 1 1] Used by Child Actor VFX and ABP
)

(event `UpdateSpeed`
  ;[1 1 1] Udpates Speed based on Engine Thrust
  (`self.UpdateEngineThrust`)
  (`self.Update Forward Velocity`))

(event `UpdateTurn`
  (params (Value :type "Float (double-precision)"))
  ;[1 1 1] Calculates Turning of the ship
  (set `self.TurnValue` Value)
  (set `self.TurnFinal` (* (`self.TurnValue`) (`self.TurnRatio`) (/ (`self.CurrentSpeed`) (`self.MaxForwardVelocity`))))
  (`self.SetTurn` (`self.TurnValue`))
  (`PrimitiveComponent.AddAngularImpulseInDegrees` (`self.SkeletalMesh`) (`KismetMathLibrary.MakeVector` 0.0 0.0 (`self.TurnFinal`)) "None" true))

(event `SetTurn`
  (params (Value :type "Float (double-precision)"))
  ;[1 1 1] Used by Child Actor VFX and ABP
)

(event `UpdateDive`
  (params (Value :type "Float (double-precision)"))
  ;[1 1 1] Dive/Submerge (Submarines only)
  (set `self.DiveValue` (* Value -1.0))
  (if (`self.isSubmarine`)
    (`self.Float Ballast Tanks` (`self.DiveValue`))))

(event `UpdatePitch`
  (params (Value :type "Float (double-precision)"))
  ;[1 1 1] Change Pitch based on Fins (Submarines only) - To be implemented in future
  (set `self.PitchValue` Value)
  (if (`self.isSubmarine`)
    (set `self.PitchFinal` (* (`self.PitchValue`) (`self.PitchRatio`) 1.0))
    (`PrimitiveComponent.AddAngularImpulseInDegrees` (`self.SkeletalMesh`) (`KismetMathLibrary.MakeVector` 0.0 (`self.PitchFinal`)) "None" true)))

(event `self.Buoyancy.OnEnteredWaterDelegate`
  (params (Pontoon :type "SphericalPontoon Structure (by ref)"))
  ;[1 1 1] Sets Water Level Z
  (bind (_outwaterplanelocation _outwaterplanenormal _outwatersurfaceposition) (`BuoyancyComponent.GetLastWaterSurfaceInfo` (`self.Buoyancy`)))
  (set `self.SurfaceLevel` (.z _outwatersurfaceposition)))

(event `InputAxis|Thrust`
  (params (AxisValue :type "Float (single-precision)"))
  ;[1 1 1] Mapps Project Inputs to coresponding Events
  (`self.UpdateThrottle` AxisValue))

(event `InputAxis|MoveRight`
  (params (AxisValue :type "Float (single-precision)"))
  ;[1 1 1] Mapps Project Inputs to coresponding Events
  (`self.UpdateTurn` AxisValue))

(event `InputAxis|Lift`
  (params (AxisValue :type "Float (single-precision)"))
  ;[1 1 1] Mapps Project Inputs to coresponding Events
  (`self.UpdateDive` AxisValue))

(event `InputAxis|Pitch`
  (params (AxisValue :type "Float (single-precision)"))
  ;[1 1 1] Mapps Project Inputs to coresponding Events
  (`self.UpdatePitch` AxisValue))

(fn `Float Ballast Tanks`
  (params (Value :type "Float (double-precision)"))
  ;[1 1 1] Fill/Empty Ballast Tanks
  (bind _output_get (set `self.BallastTanksValue` (`KismetMathLibrary.FClamp` (+ (* Value (`self.BallastTanksFillRatio`)) (`self.BallastTanksValue`)) (`self.BallastTanksMinCapacity`) (`self.BallastTanksMaxCapacity`))))
  (`PrimitiveComponent.SetMassOverrideInKg` (`self.SkeletalMesh`) "None" _output_get true))

(fn `Update Forward Velocity`
  (bind _x (.x (`SceneComponent.GetComponentVelocity` (`self.SkeletalMesh`))))
  ;[1 1 1] Updates Forwards Backwards Speed
  (set `self.CurrentSpeed` _x)
  (if (<= (`KismetMathLibrary.Abs` _x) (`self.MaxForwardVelocity`))
    (`PrimitiveComponent.AddForce` (`self.SkeletalMesh`) (`KismetMathLibrary.GreaterGreater_VectorRotator` (`KismetMathLibrary.MakeVector` (`self.EngineThrust`)) (`self.K2_GetActorRotation`)) "None" true)))

(fn `UpdateEngineThrust`
  ;[1 1 1] Updates Thrust based on Throttle
  (set `self.EngineThrust` (* (`self.Throttle`) 100.0)))

(fn `UserConstructionScript`
  (`parent.UserConstructionScript`))