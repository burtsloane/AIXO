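; Base water vehicle Blueprint for player-driven ships and submarines, moved by ProjectileMovement instead of physics simulation.
; Axis inputs set throttle, turn and submarine-only dive and pitch, which Tick turns into local-space velocity and actor rotation.
; Starting Z serves as sea level, limiting depth and pitch, while timelines fake wave roll.
; Front, rear and bottom capsules block movement and push physics objects; spawned projectiles inherit vehicle velocity.
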(event `self.ReceiveBeginPlay`
  (`parent.ReceiveBeginPlay`)
  ;[1 1 1] Considers Initial Z position as Water Surface level
  (set `self.SurfaceLevel` (.z (`self.K2_GetActorLocation`)))
  ;[1 1 1] Initiates fake Water Waves Impact
  (`TimelineComponent.SetPlayRate` (`self.WavesPitch`) 0.1)
  (`TimelineComponent.SetPlayRate` (`self.WavesRoll`) 0.15)
  (`self.StartWaves`))

(event `self.ReceiveTick`
  (params (DeltaSeconds :type "Float (single-precision)"))
  (`parent.ReceiveTick` DeltaSeconds)
  ;[1 1 1] Updates Speed and Rotation
  (`self.UpdateSpeed`)
  (`self.K2_SetActorRotation` (`KismetMathLibrary.MakeRotator` (`self.VawesRollValue`) (`self.FinalPitch`) (`self.TurnFinal`))))

(event `UpdateThrottle`
  (params (Value :type "Float (double-precision)"))
  ;[1 1 1] Updates Throttle
  (set `self.Throttle` (`KismetMathLibrary.FClamp` (+ (* Value (`self.ThrottleRate`)) (`self.Throttle`)) -1.0))
  (`self.SetThrottle` (`self.Throttle`)))

(event `SetThrottle`
  (params (Value :type "Float (double-precision)"))
  ;[1 1 1] Used by Child Actor VFX and ABP
)

(event `UpdateSpeed`
  ;[1 1 1] Updates Thurst Velocity and Depth
  (`self.UpdateEngineThrust`)
  (`self.Update Forward Velocity`)
  (`self.UpdateDepth`)
  ;[1 1 1] Provides final velocity values for Projectile Movement
  (`ProjectileMovementComponent.SetVelocityInLocalSpace` (`self.ProjectileMovement`) (+ (`KismetMathLibrary.MakeVector` (`self.ForwardSpeed`)) (`KismetMathLibrary.InverseTransformDirection` (`self.GetTransform`) (`KismetMathLibrary.MakeVector` 0.0 0.0 (`self.VerticalVelocity`))))))

(event `Update Turn`
  (params (Value :type "Float (double-precision)"))
  ;[1 1 1] Calculates Turning of the ship
  (set `self.TurnValue` Value)
  (`self.SetTurn` (`self.TurnValue`))
  (set `self.TurnFinal` (+ (.yaw (`self.K2_GetActorRotation`)) (* (`self.TurnValue`) (`self.Turn_Rate`) (/ (`self.ForwardSpeed`) (`self.MarginalVelocity`))))))

(event `SetTurn`
  (params (Value :type "Float (double-precision)"))
  ;[1 1 1] Used by Child Actor VFX and ABP
)

(event `UpdateDive`
  (params (Value :type "Float (double-precision)"))
  ;[1 1 1] Updates Dive/Submerge Value (Submarines only)
  (if (`self.isSubmarine`)
    (set `self.DivingValue` Value)))

(event `UpdatePitch`
  (params (Value :type "Float (double-precision)"))
  ;[1 1 1] Calculates Pitch based on Fins Position (Submarines only)
  (set `self.Pitch` Value)
  (if (`self.isSubmarine`)
    (`self.CalculatePitch`)))

(event `StartWaves`
  ;[1 1 1] Simulate fake waves impact
  (`|ExecutionSequence`
    (:`then_0`
      (bind (_direction _cu_sinus) (`Timeline|WavesPitch` :!label _label)
        (:`Update`
          (set `self.VawesPitchValue` (* _cu_sinus 2.0)))))
    (:`then_1`
      (bind (_direction_2 _cu_sinus_2) (`Timeline|WavesRoll` :!label _label_2)
        (:`Update`
          (set `self.VawesRollValue` (* _cu_sinus_2 5.0)))))))

(event `SetPitch`
  (params (Value :type "Float (double-precision)"))
  ;[1 1 1] Used by Child Actor VFX and ABP
)

(event `StopWaves`
  ;[1 1 1] Simulate fake waves impact
  (`|ExecutionSequence`
    (:`then_0`
      (goto _label :!via `Stop`))
    (:`then_1`
      (goto _label_2 :!via `Stop`))))

(event `self.FrontCapsule.OnComponentBeginOverlap`
  (params (OverlappedComponent :type "PrimitiveComponent Object Reference") (OtherActor :type "Actor Object Reference") (OtherComp :type "PrimitiveComponent Object Reference") (OtherBodyIndex :type Integer) (bFromSweep :type Boolean) (SweepResult :type "HitResult Structure (by ref)"))
  ;[1 1 1] Detects Collisions with obstacles
  (cast `WaterBodyOcean` OtherActor
    (:`CastFailed`
      (cast `/Game/VigilanteMovement/Vehicles/West_SSN_LosAngeles/BP_West_SSN_LosAngeles_Projectile` OtherActor
        (:`CastFailed`
          (`self.BounceObstacle` OtherComp)
          (set `self.FwdBlocked` true))))))

(event `self.FrontCapsule.OnComponentEndOverlap`
  (params (OverlappedComponent :type "PrimitiveComponent Object Reference") (OtherActor :type "Actor Object Reference") (OtherComp :type "PrimitiveComponent Object Reference") (OtherBodyIndex :type Integer))
  ;[1 1 1] Detects Collisions with obstacles
  (cast `WaterBodyOcean` OtherActor
    (:`CastFailed`
      (cast `/Game/VigilanteMovement/Vehicles/West_SSN_LosAngeles/BP_West_SSN_LosAngeles_Projectile` OtherActor
        (:`CastFailed`
          (set `self.FwdBlocked` false))))))

(event `self.RearCapsule.OnComponentBeginOverlap`
  (params (OverlappedComponent :type "PrimitiveComponent Object Reference") (OtherActor :type "Actor Object Reference") (OtherComp :type "PrimitiveComponent Object Reference") (OtherBodyIndex :type Integer) (bFromSweep :type Boolean) (SweepResult :type "HitResult Structure (by ref)"))
  ;[1 1 1] Detects Collisions with obstacles
  (cast `WaterBodyOcean` OtherActor
    (:`CastFailed`
      (cast `/Game/VigilanteMovement/Vehicles/West_SSN_LosAngeles/BP_West_SSN_LosAngeles_Projectile` OtherActor
        (:`CastFailed`
          (`self.BounceObstacle` OtherComp)
          (set `self.RearBlocked` true))))))

(event `self.RearCapsule.OnComponentEndOverlap`
  (params (OverlappedComponent :type "PrimitiveComponent Object Reference") (OtherActor :type "Actor Object Reference") (OtherComp :type "PrimitiveComponent Object Reference") (OtherBodyIndex :type Integer))
  ;[1 1 1] Detects Collisions with obstacles
  (cast `WaterBodyOcean` OtherActor
    (:`CastFailed`
      (cast `/Game/VigilanteMovement/Vehicles/West_SSN_LosAngeles/BP_West_SSN_LosAngeles_Projectile` OtherActor
        (:`CastFailed`
          (set `self.RearBlocked` false))))))

(event `self.BottomCapsule.OnComponentBeginOverlap`
  (params (OverlappedComponent :type "PrimitiveComponent Object Reference") (OtherActor :type "Actor Object Reference") (OtherComp :type "PrimitiveComponent Object Reference") (OtherBodyIndex :type Integer) (bFromSweep :type Boolean) (SweepResult :type "HitResult Structure (by ref)"))
  ;[1 1 1] Detects Collisions with obstacles
  (cast `WaterBodyOcean` OtherActor
    (:`CastFailed`
      (cast `/Game/VigilanteMovement/Vehicles/West_SSN_LosAngeles/BP_West_SSN_LosAngeles_Projectile` OtherActor
        (:`CastFailed`
          (`self.BounceObstacle` OtherComp)
          (set `self.BottomBlocked` true))))))

(event `self.BottomCapsule.OnComponentEndOverlap`
  (params (OverlappedComponent :type "PrimitiveComponent Object Reference") (OtherActor :type "Actor Object Reference") (OtherComp :type "PrimitiveComponent Object Reference") (OtherBodyIndex :type Integer))
  ;[1 1 1] Detects Collisions with obstacles
  (cast `WaterBodyOcean` OtherActor
    (:`CastFailed`
      (cast `/Game/VigilanteMovement/Vehicles/West_SSN_LosAngeles/BP_West_SSN_LosAngeles_Projectile` OtherActor
        (:`CastFailed`
          (set `self.BottomBlocked` false))))))

(event `InputAxis|Thrust`
  (params (AxisValue :type "Float (single-precision)"))
  ;[1 1 1] Mapps Project Inputs to coresponding Events
  (`self.UpdateThrottle` AxisValue))

(event `InputAxis|MoveRight`
  (params (AxisValue :type "Float (single-precision)"))
  ;[1 1 1] Mapps Project Inputs to coresponding Events
  (`self.Update Turn` AxisValue))

(event `InputAxis|Lift`
  (params (AxisValue :type "Float (single-precision)"))
  ;[1 1 1] Mapps Project Inputs to coresponding Events
  (`self.UpdateDive` AxisValue))

(event `InputAxis|Pitch`
  (params (AxisValue :type "Float (single-precision)"))
  ;[1 1 1] Mapps Project Inputs to coresponding Events
  (`self.UpdatePitch` AxisValue))

(fn `BounceObstacle`
  (params (Target :type "PrimitiveComponent Object Reference"))
  ;[1 1 1] Applies Physics Forse on Objects on Bounce
  (if (`SceneComponent.IsSimulatingPhysics` Target "None")
    (`PrimitiveComponent.AddImpulse` Target (* (`MovementComponent.Velocity` (`self.ProjectileMovement`)) 2.0) "None" true)))

(fn `CalculatePitch`
  (bind _returnvalue (+ (.pitch (`self.K2_GetActorRotation`)) (`self.Pitch`)))
  ;[1 1 1] Calculates the Pitch based on Direction and Distance to the Surface
  (if (> (`self.ForwardSpeed`) 0.0)
    (set `self.FinalPitch` (`KismetMathLibrary.FClamp` _returnvalue (`KismetMathLibrary.FClamp` (* (- (`self.SurfaceLevel`) (.z (`self.K2_GetActorLocation`))) -0.01) -30.0 -2.5) (`KismetMathLibrary.FClamp` (* (- (`self.SurfaceLevel`) (.z (`self.K2_GetActorLocation`))) 0.2) 0.0 30.0)))
    (elif (< (`self.ForwardSpeed`) 0.0)
      (set `self.FinalPitch` (`KismetMathLibrary.FClamp` _returnvalue (`KismetMathLibrary.FClamp` (* (- (`self.SurfaceLevel`) (.z (`self.K2_GetActorLocation`))) -0.01) -30.0 0.0) (`KismetMathLibrary.FClamp` (* (- (`self.SurfaceLevel`) (.z (`self.K2_GetActorLocation`))) 0.02) 2.5 30.0)))
      (else
        (set `self.FinalPitch` 0.0))))
  (`self.SetPitch` (`self.Pitch`)))

(fn `InitProjectile`
  (params (BaseProjectileMovement :type "ProjectileMovementComponent Object Reference"))
  (`parent.InitProjectile` BaseProjectileMovement)
  (set `MovementComponent.Velocity` (`MovementComponent.Velocity` (`self.ProjectileMovement`)) BaseProjectileMovement))

(fn `Update Forward Velocity`
  ;[1 1 1] Updates Forwards Backwards Speed
  (set `self.ForwardSpeed` (`KismetMathLibrary.FClamp` (+ (`self.ForwardSpeed`) (* (`self.Throttle`) (`self.AccelerationRate`))) (* (`self.MarginalVelocity`) -1.0) (`self.MarginalVelocity`)))
  ;[1 1 1] Blocks Movement on Collision
  (if (> (`self.Throttle`) 0.0)
    (if (`self.FwdBlocked`)
      (set `self.ForwardSpeed` 0.0 :!label _label))
    (elif (< (`self.Throttle`) 0.0)
      (if (`self.RearBlocked`)
        (goto _label)))))

(fn `UpdateDepth`
  ;[1 1 1] Checks if on Surface
  (if (> (`self.SurfaceLevel`) (.z (`self.K2_GetActorLocation`)))
    ;[1 1 1] Checks for Diving Blocking Collisions
    (if (< (`self.DivingValue`) 0.0)
      (if (`self.BottomBlocked`)
        (set `self.DivingValue` 0.0)))
    ;[1 1 1] Updates Dive/Surface Velocity
    (set `self.VerticalVelocity` (* (`self.DivingValue`) (`self.DivingRate`)) :!label _label)
    ;[1 1 1] Toggles Fake Waves if on surface
    (if (`self.isSurface`)
      (`self.StopWaves`)
      (set `self.isSurface` false))
    (elif (< (`self.DivingValue`) 0.0)
      (goto _label)
      (else
        (set `self.VerticalVelocity` 0.0)
        (if (not (`self.isSurface`))
          (`self.StartWaves`)
          (set `self.isSurface` false))))))

(fn `UpdateEngineThrust`
  ;[1 1 1] Updates Thrust based on Throttle
  (set `self.EngineThrust` (`self.Throttle`)))

(fn `UserConstructionScript`
  (`parent.UserConstructionScript`))