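; Showcase Blueprint for the Los Angeles-class submarine that exposes its controls through generic slider, button and checkbox events.
; Sliders drive throttle, turn, pitch, snorkel and nav radar, while twin sliders set right and left periscopes and antennas.
; Button indices open or close shafts and start or stop firing, and a checkbox toggles damaged mode.
; Each event only forwards to the submarine's own functions, with no added logic.
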(event `/Game/VigilanteMovement/Shared/Blueprints/HUD/Showcase/Interfaces/BP_ShowcaseControlsInterface.SetSliderVariable0`
  (params (NewValue :type "Float (double-precision)"))
  (`self.SetThrottle` NewValue))

(event `/Game/VigilanteMovement/Shared/Blueprints/HUD/Showcase/Interfaces/BP_ShowcaseControlsInterface.SetSliderVariable1`
  (params (NewValue :type "Float (double-precision)"))
  (`self.SetTurn` NewValue))

(event `/Game/VigilanteMovement/Shared/Blueprints/HUD/Showcase/Interfaces/BP_ShowcaseControlsInterface.SetSliderVariable2`
  (params (NewValue :type "Float (double-precision)"))
  (`self.SetPitch` NewValue))

(event `/Game/VigilanteMovement/Shared/Blueprints/HUD/Showcase/Interfaces/BP_ShowcaseControlsInterface.SetSliderVariable3`
  (params (NewValue :type "Float (double-precision)"))
  (`self.SetSnorkel` NewValue))

(event `/Game/VigilanteMovement/Shared/Blueprints/HUD/Showcase/Interfaces/BP_ShowcaseControlsInterface.SetSliderVariable4`
  (params (NewValue :type "Float (double-precision)"))
  (`self.SetNavRadar` NewValue))

(event `/Game/VigilanteMovement/Shared/Blueprints/HUD/Showcase/Interfaces/BP_ShowcaseControlsInterface.SetTwinSliderVariable0`
  (params (`bFirstSlider?` :type Boolean) (NewFirstValue :type "Float (double-precision)") (NewSecondValue :type "Float (double-precision)"))
  (`self.SetPeriscopes` NewFirstValue NewSecondValue))

(event `/Game/VigilanteMovement/Shared/Blueprints/HUD/Showcase/Interfaces/BP_ShowcaseControlsInterface.SetTwinSliderVariable1`
  (params (`bFirstSlider?` :type Boolean) (NewFirstValue :type "Float (double-precision)") (NewSecondValue :type "Float (double-precision)"))
  (`self.SetAntennas` NewFirstValue NewSecondValue))

(event `/Game/VigilanteMovement/Shared/Blueprints/HUD/Showcase/Interfaces/BP_ShowcaseControlsInterface.SetButtonsVariable0`
  (params (NewIndex :type Integer))
  (switch `int` NewIndex
    (:`0`
      (`self.OpenShafts`))
    (:`1`
      (`self.CloseShafts`))))

(event `/Game/VigilanteMovement/Shared/Blueprints/HUD/Showcase/Interfaces/BP_ShowcaseControlsInterface.SetButtonsVariable1`
  (params (NewIndex :type Integer))
  (switch `int` NewIndex
    (:`0`
      (`self.StartFire`))
    (:`1`
      (`self.StopFire`))))

(event `/Game/VigilanteMovement/Shared/Blueprints/HUD/Showcase/Interfaces/BP_ShowcaseControlsInterface.SetCheckboxVariable0`
  (params (NewState :type Boolean))
  (`self.SetDamagedMode` NewState))

(fn `UserConstructionScript`
  (`parent.UserConstructionScript`))