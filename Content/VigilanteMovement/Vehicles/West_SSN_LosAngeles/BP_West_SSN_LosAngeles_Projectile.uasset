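; Los Angeles-class submarine Blueprint that animates the hull and gates the parent's firing on open missile shafts.
; Throttle, turn and pitch events drive the ABP's propeller, rudders and hydroplanes, with propeller depth below SurfaceLevel switching Niagara bubbles and surface splash.
; Input FlipFlops run reversible timelines that open the shafts and raise the snorkel, periscopes and antennas.
; StartFire is overridden to fire only after the shafts finish opening.
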(event `self.ReceiveBeginPlay`
  (`parent.ReceiveBeginPlay`)
  ;[1 1 1] Sets ABP Reference
  (bind _asabp_west_ssn_los_angeles (cast `/Game/VigilanteMovement/Vehicles/West_SSN_LosAngeles/ABP_West_SSN_LosAngeles` (`SkeletalMeshComponent.GetAnimInstance` (`self.SkeletalMesh`))))
  (set `self.AnimInstance` _asabp_west_ssn_los_angeles)
  ;[1 1 1] Retracts Equipment on Begin
  (`self.SetSnorkel` 0.0)
  (`self.SetPeriscopes` 0.0)
  (`self.SetAntennas` 0.0))

(event `self.SetThrottle`
  (params (Value :type "Float (double-precision)"))
  (bind _propellerdepth (`self.PropellerDepth`))
  ;[1 1 1] Updates Propeller Speed
  (set `/Game/VigilanteMovement/Vehicles/West_SSN_LosAngeles/ABP_West_SSN_LosAngeles.PropellerSpeed` (* Value 500.0) (`self.AnimInstance`))
  (`NiagaraComponent.SetVariableFloat` (`self.NS_West_SSN_LosAngeles_Prop`) "PropSpeed" (* (`KismetMathLibrary.Abs` Value) 400.0))
  (set `self.PropellerDepth` (- (`self.SurfaceLevel`) (.z (`SceneComponent.GetSocketLocation` (`self.SkeletalMesh`) "propeller"))))
  (if (> (`self.PropellerDepth`) 1200.0)
    (`NiagaraComponent.SetVariableFloat` (`self.NS_West_SSN_LosAngeles_Prop`) "Bubbles" 1.0)
    (`NiagaraComponent.SetVariableFloat` (`self.NS_West_SSN_LosAngeles_Prop`) "SurfaceSplash" 0.0)
    (else
      (`NiagaraComponent.SetVariableFloat` (`self.NS_West_SSN_LosAngeles_Prop`) "Bubbles" 0.0)
      (`NiagaraComponent.SetVariableFloat` (`self.NS_West_SSN_LosAngeles_Prop`) "SurfaceSplash" 1.0)
      (if (> _propellerdepth 650.0)
        (`NiagaraComponent.SetVariableFloat` (`self.NS_West_SSN_LosAngeles_SurfacingSplash`) "PropDepth" 0.0)
        (else
          (`NiagaraComponent.SetVariableFloat` (`self.NS_West_SSN_LosAngeles_SurfacingSplash`) "PropDepth" (* _propellerdepth 3.0)))))))

(event `self.SetTurn`
  (params (Value :type "Float (double-precision)"))
  (bind _returnvalue (* Value -1.0))
  ;[1 1 1] Updates Rudders Position
  (`/Game/VigilanteMovement/Vehicles/West_SSN_LosAngeles/ABP_West_SSN_LosAngeles.SetRearRudder` (`self.AnimInstance`) _returnvalue _returnvalue))

(event `self.SetPitch`
  (params (Value :type "Float (double-precision)"))
  ;[1 1 1] Updates Hydroplane Fins
  (`/Game/VigilanteMovement/Vehicles/West_SSN_LosAngeles/ABP_West_SSN_LosAngeles.SetFrontHydroplane` (`self.AnimInstance`) Value Value)
  (`/Game/VigilanteMovement/Vehicles/West_SSN_LosAngeles/ABP_West_SSN_LosAngeles.SetRearHydroplane` (`self.AnimInstance`) Value Value))

(event `OpenShafts`
  ;[1 1 1] Opens/Closes Shafts and enables fire
  (set `self.FireReady` false)
  (`self.StopFire`)
  (bind (_direction _cu_smooth_simplecurve) (`Timeline|UpdateShafts` :!label _label)
    (:`Update`
      (`/Game/VigilanteMovement/Vehicles/West_SSN_LosAngeles/ABP_West_SSN_LosAngeles.SetMissileShaftAngles` (`self.AnimInstance`) _cu_smooth_simplecurve _cu_smooth_simplecurve))
    (:`Finished`
      (if (`|EnumEquality` _direction "Forward")
        (set `self.FireReady` true)))))

(event `CloseShafts`
  ;[1 1 1] Opens/Closes Shafts and enables fire
  (set `self.FireReady` false)
  (`self.StopFire`)
  (goto _label :!via `Reverse`))

(event `InputAction|Open Canopy`
  (params (Key :type "Key Structure"))
  ;[1 1 1] Toggles Shafts
  (:`Pressed`
    (`/Engine/EditorBlueprintResources/StandardMacros.FlipFlop`
      (:`A`
        (`self.OpenShafts`))
      (:`B`
        (`self.CloseShafts`)))))

(event `SetSnorkel`
  (params (Value :type "Float (double-precision)"))
  ;[1 1 1] Sets Snorkel position
  (`/Game/VigilanteMovement/Vehicles/West_SSN_LosAngeles/ABP_West_SSN_LosAngeles.SetSnorkel` (`self.AnimInstance`) Value))

(event `SetNavRadar`
  (params (Value :type "Float (double-precision)"))
  ;[1 1 1] Sets Radar Angle
  (`/Game/VigilanteMovement/Vehicles/West_SSN_LosAngeles/ABP_West_SSN_LosAngeles.SetNavigationalRadar` (`self.AnimInstance`) Value))

(event `SetPeriscopes`
  (params (ValueRight :type "Float (double-precision)") (ValueLeft :type "Float (double-precision)"))
  ;[1 1 1] Sets Periscopes Position
  (`/Game/VigilanteMovement/Vehicles/West_SSN_LosAngeles/ABP_West_SSN_LosAngeles.SetPeriscopes` (`self.AnimInstance`) ValueRight ValueLeft))

(event `SetAntennas`
  (params (ValueRight :type "Float (double-precision)") (ValueLeft :type "Float (double-precision)"))
  ;[1 1 1] Sets Antennas Position
  (`/Game/VigilanteMovement/Vehicles/West_SSN_LosAngeles/ABP_West_SSN_LosAngeles.SetRadioAntennas` (`self.AnimInstance`) ValueRight ValueLeft))

(event `InputAction|Hook`
  (params (Key :type "Key Structure"))
  ;[1 1 1] Toggles Equipment
  (:`Pressed`
    (`/Engine/EditorBlueprintResources/StandardMacros.FlipFlop`
      (:`A`
        (bind (_direction _cu_smooth_simplecurve) (`Timeline|UpdateEquipment` :!via `PlayFromStart` :!label _label_2)
          (:`Update`
            (`self.SetSnorkel` _cu_smooth_simplecurve)
            (`self.SetPeriscopes` _cu_smooth_simplecurve _cu_smooth_simplecurve)
            (`self.SetAntennas` _cu_smooth_simplecurve _cu_smooth_simplecurve))))
      (:`B`
        (goto _label_2 :!via `ReverseFromEnd`)))))

(fn `StartFire`
  ;[1 1 1] Overrides Parent funtion to fire only if Shafts are open
  (if (`self.FireReady`)
    (`parent.StartFire`)
    (else
      (`self.StopFire`))))

(fn `UserConstructionScript`
  (`parent.UserConstructionScript`))