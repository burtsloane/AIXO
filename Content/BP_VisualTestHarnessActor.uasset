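; Test harness actor that runs a Llama language-model component and relays its output to CommandTester.
; BeginPlay activates Llama and binds its new-token, full-context-dump and tool-call events.
; Tokens and context dumps both go to CommandTester's AIXOToken, while tool-call JSON is only printed.
; RequestContextDump triggers a full context dump on demand; a startup ProcessInput call is left disconnected.
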(event `self.ReceiveBeginPlay`
  (`ActorComponent.Activate` (`self.Llama`) false)
  (add `LlamaComponent.OnNewTokenGenerated` (`self.Llama`) (delegate `NewTokenGenerated`))
  (add `LlamaComponent.OnFullContextDumpReady` (`self.Llama`) (delegate `NewTextGenerated`))
  (add `LlamaComponent.OnToolCallDetected` (`self.Llama`) (delegate `ToolCall`)))

(event `NewTokenGenerated`
  (params (NewToken :type String))
  (`/Game/WBP_CommandTester.AIXOToken` (`self.CommandTester`) NewToken))

(event `NewTextGenerated`
  (params (ContextDump :type String))
  (`/Game/WBP_CommandTester.AIXOToken` (`self.CommandTester`) ContextDump))

(event `ToolCall`
  (params (ToolCallJson :type String))
  (`KismetSystemLibrary.PrintString` ToolCallJson))

(event `RequestContextDump`
  (`LlamaComponent.TriggerFullContextDump` (`self.Llama`)))

(fn `UserConstructionScript`)